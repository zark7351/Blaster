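; Behavior tree task that moves an AI controller to a chase location read from the blackboard.
; On execute it runs AI Move To toward the Lco vector key, finishing with success on arrival or failure if the request fails.
; Both outcomes and an abort clear the Chase blackboard key before the task ends.
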(event EventReceiveExecuteAI
  (params (OwnerController :type AI%20Controller%20Object%20Reference) (ControlledPawn :type Pawn%20Object%20Reference))
  (AI|AIMoveTo OwnerController (Class|BTFunctionLibrary|GetBlackboardValueasVector (Variables|Default|GetLco)) 0 5e+01 "Default" "Default" true true
    (:OnRequestFailed
      (Class|BTFunctionLibrary|ClearBlackboardValue (Variables|Default|GetChase))
      (AI|BehaviorTree|FinishExecute false))
    (:OnMoveFinished
      (Class|BTFunctionLibrary|ClearBlackboardValue (Variables|Default|GetChase))
      (AI|BehaviorTree|FinishExecute true))))

(event EventReceiveAbortAI
  (params (OwnerController :type AI%20Controller%20Object%20Reference) (ControlledPawn :type Pawn%20Object%20Reference))
  (Class|BTFunctionLibrary|ClearBlackboardValue (Variables|Default|GetChase))
  (Class|BTTaskBlueprintBase|FinishAbort))