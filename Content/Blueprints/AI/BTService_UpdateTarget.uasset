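; Behavior tree service that keeps an AI pawn's aim Target updated to the head of the character stored in a blackboard key.
; On each AI tick it casts the controlled pawn to the Blaster, Mina or PinkGirl AI class in turn.
; If the key holds a BlasterCharacter, it writes that mesh's HeadSocket location into the pawn's Target variable, duplicating the logic per class.
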(event EventReceiveTickAI
  (params (OwnerController :type AI%20Controller%20Object%20Reference) (ControlledPawn :type Pawn%20Object%20Reference) (DeltaSeconds :type Float%20%28single-precision%29))
  (bind _key (Variables|Default|GetKey))
  (bind _returnvalue (Class|BTFunctionLibrary|GetBlackboardValueasObject _key))
  (bind (_asblaster_character _bsuccess) (Utilities|Casting|CastToBlasterCharacter _returnvalue))
  (bind _mesh (Variables|/Script/Engine.Character|GetMesh _asblaster_character))
  (bind _returnvalue_2 (Transformation|GetSocketLocation _mesh "HeadSocket"))
  (bind _asbp_aiblaster (Utilities|Casting|CastToBP_AIBlaster ControlledPawn)
    (:then
      (if _bsuccess
        (Variables|/Game/Blueprints/Character/BP_AIBlaster.BP_AIBlaster_C|SetTarget _asbp_aiblaster _returnvalue_2)))
    (:CastFailed
      (bind _asbp_aimina (Utilities|Casting|CastToBP_AIMina ControlledPawn)
        (:then
          (if _bsuccess
            (Variables|/Game/Blueprints/Character/BP_AIMina.BP_AIMina_C|SetTarget _asbp_aimina _returnvalue_2)))
        (:CastFailed
          (bind _asbp_aipink_girl (Utilities|Casting|CastToBP_AIPinkGirl ControlledPawn))
          (if _bsuccess
            (Variables|/Game/Blueprints/Character/BP_AIPinkGirl.BP_AIPinkGirl_C|SetTarget _asbp_aipink_girl _returnvalue_2)))))))