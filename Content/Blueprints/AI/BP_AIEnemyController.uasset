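; AI controller for enemy BlasterCharacters that runs the BT_Enemy behavior tree and feeds it from AI Perception.
; Sensing a non-AI character stores it as the target and sets HasTarget on the pawn's Combat component.
; Losing it clears both, saves the lost location and sets a weighted-random Chase flag, usually true.
; Perception info updates also write any BlasterCharacter's location to the blackboard.
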(event OnTargetPerceptionUpdated(AIPerception)
  (params (Actor :type Actor%20Object%20Reference) (Stimulus :type AI%20Stimulus%20Structure))
  (bind _returnvalue (Pawn|GetControlledPawn))
  (bind _returnvalue_2 (AI|GetBlackboard 0))
  (bind _obj (Variables|Default|GetObj))
  (bind _chase (Variables|Default|GetChase))
  (bind _lostlocation (Variables|Default|GetLostLocation))
  (bind _asblaster_character (Utilities|Casting|CastToBlasterCharacter Actor))
  (if (not (Variables|/Script/Blaster.BlasterCharacter|GetIsAI _asblaster_character))
    (if (.bsuccessfullysensed Stimulus)
      (AI|Components|Blackboard|SetValueasObject _returnvalue_2 _obj _asblaster_character)
      (AI|Components|Blackboard|ClearValue _returnvalue_2 _chase)
      (AI|Components|Blackboard|ClearValue _returnvalue_2 _lostlocation)
      (bind _asblaster_character_2 (Utilities|Casting|CastToBlasterCharacter _returnvalue))
      (Variables|/Script/Blaster.CombatComponent|SetbHasTarget (Variables|/Script/Blaster.BlasterCharacter|GetCombat _asblaster_character_2) true)
      (else
        (AI|Components|Blackboard|ClearValue _returnvalue_2 _obj)
        (AI|Components|Blackboard|SetValueasBool _returnvalue_2 _chase (Math|Random|RandomBoolwithWeight 0.8))
        (AI|Components|Blackboard|SetValueasVector _returnvalue_2 _lostlocation (Transformation|GetActorLocation _asblaster_character))
        (bind _asblaster_character_3 (Utilities|Casting|CastToBlasterCharacter _returnvalue))
        (Variables|/Script/Blaster.CombatComponent|SetbHasTarget (Variables|/Script/Blaster.BlasterCharacter|GetCombat _asblaster_character_3) false)))))

(event OnTargetPerceptionInfoUpdated(AIPerception)
  (params (UpdateInfo :type Actor%20Perception%20Update%20Info%20Structure%20%28by%20ref%29))
  (bind _asblaster_character (Utilities|Casting|CastToBlasterCharacter (.target UpdateInfo)))
  (AI|Components|Blackboard|SetValueasVector (AI|GetBlackboard 0) (Variables|Default|GetLoc) (Transformation|GetActorLocation _asblaster_character)))

(event EventBeginPlay
  (AI|RunBehaviorTree "/Game/Blueprints/AI/BT_Enemy.BT_Enemy"))

(fn ConstructionScript)