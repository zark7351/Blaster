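; BP_AIPinkGirl is an AI-driven character that turns to face and aim at its combat target.
; While the Combat component has a target, Tick copies Target into HitTarget and smoothly interpolates controller and actor yaw toward it.
; It also stores the yaw difference in AOYaw, likely for an aim offset.
; The construction script destroys components tagged UseForPlayer, stripping player-only parts from the AI.
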(event EventTick
  (params (DeltaSeconds :type Float%20%28single-precision%29))
  (bind _returnvalue (Transformation|GetActorLocation))
  (bind _returnvalue_2 (Transformation|GetActorRotation))
  (bind _target (Variables|Default|GetTarget))
  (bind _combat (Variables|Default|GetCombat))
  (bind _returnvalue_3 (Math|Rotator|FindLookatRotation _returnvalue _target))
  (bind _returnvalue_4 (Math|Interpolation|RInterpTo _returnvalue_2 _returnvalue_3 DeltaSeconds 4.0))
  (Utilities|FlowControl|Sequence
    (:then_1
      (if (Variables|/Script/Blaster.CombatComponent|GetbHasTarget _combat)
        (Variables|/Script/Blaster.CombatComponent|SetHitTarget _combat _target)
        (Pawn|SetControlRotation (Pawn|GetController) (Math|Rotator|MakeRotator 0.0 0.0 (.yaw _returnvalue_4)))
        (Variables|Default|SetAO_Yaw (.yaw (Math|Rotator|Delta(Rotator) _returnvalue_3 _returnvalue_2)))
        (Transformation|SetActorRotation (Math|Rotator|MakeRotator 0.0 0.0 (.yaw _returnvalue_4)))))))

(fn ConstructionScript
  (for _array_element (Actor|GetComponentsbyTag "/Script/Engine.ActorComponent" "UseForPlayer")
    (Components|DestroyComponent _array_element)))